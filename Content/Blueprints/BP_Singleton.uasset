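; BP_Singleton handles per-level persistence of collected objects, with load, save and delete events that use the current level name as the slot.
; Load waits briefly, clears PreviouslyCollectedObjs, then destroys each actor listed in the level's SG_Objects save without refilling that array.
; Save reuses or creates the save object and overwrites its CollectedObjs with PreviouslyCollectedObjs.
; DeleteSave removes the level's slot if it exists.
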(event `Load`
  (`KismetSystemLibrary.PrintString` "Doing The Loading Thing")
  (`KismetSystemLibrary.Delay` 0.2)
  (bind _returnvalue (`GameplayStatics.GetCurrentLevelName` true))
  (`KismetArrayLibrary.Array_Clear` (`self.PreviouslyCollectedObjs`))
  (`KismetSystemLibrary.PrintString` (`KismetStringLibrary.Concat_StrStr` "Starting Load in Level " _returnvalue " wish me luck"))
  (bind _returnvalue_2 (`GameplayStatics.DoesSaveGameExist` _returnvalue))
  (if _returnvalue_2
    (bind _returnvalue_3 (`GameplayStatics.LoadGameFromSlot` _returnvalue))
    (bind _assg_objects (cast `/Game/Blueprints/SG_Objects` _returnvalue_3))
    (set `self.As SG Objects` _assg_objects)
    (for _array_element (`/Game/Blueprints/SG_Objects.CollectedObjs` _assg_objects)
      (`Actor.K2_DestroyActor` _array_element))))

(event `Save`
  (`KismetSystemLibrary.PrintString` "Doing The Save Thing")
  (bind _returnvalue (`GameplayStatics.GetCurrentLevelName` true))
  (bind _returnvalue_2 (`GameplayStatics.DoesSaveGameExist` _returnvalue))
  (if _returnvalue_2
    (bind _returnvalue_3 (`GameplayStatics.LoadGameFromSlot` _returnvalue))
    (set `self.SaveSubclass` _returnvalue_3)
    (else
      (bind _returnvalue_4 (`GameplayStatics.CreateSaveGameObject` "/Game/Blueprints/SG_Objects.SG_Objects_C"))
      (set `self.SaveSubclass` _returnvalue_4)))
  (bind _assg_objects (cast `/Game/Blueprints/SG_Objects` (`self.SaveSubclass`)))
  (set `/Game/Blueprints/SG_Objects.CollectedObjs` (`self.PreviouslyCollectedObjs`) _assg_objects)
  (bind _returnvalue_5 (`GameplayStatics.GetCurrentLevelName` true))
  (`GameplayStatics.SaveGameToSlot` _assg_objects _returnvalue_5)
  (`KismetSystemLibrary.PrintString` "Did The Save Thing"))

(event `DeleteSave`
  (bind _returnvalue (`GameplayStatics.GetCurrentLevelName` true))
  (bind _returnvalue_2 (`GameplayStatics.DoesSaveGameExist` _returnvalue))
  (if _returnvalue_2
    (`GameplayStatics.DeleteGameInSlot` _returnvalue)
    (`KismetSystemLibrary.PrintString` "Save Deleted")
    (else
      (`KismetSystemLibrary.PrintString` "No Save Game Exists"))))