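; Automatic sliding glass door for an archviz scene that opens when something overlaps its Box trigger.
; Separate timelines drive the relative location of the left and right door meshes, playing forward to open and in reverse to close.
; End overlap starts a retriggerable two-second delay before closing, then clears the DoorsOpen flag one second later so the doors can open again.
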(event `self.Box.OnComponentBeginOverlap`
  (params (OverlappedComponent :type "PrimitiveComponent Object Reference") (OtherActor :type "Actor Object Reference") (OtherComp :type "PrimitiveComponent Object Reference") (OtherBodyIndex :type Integer) (bFromSweep :type Boolean) (SweepResult :type "HitResult Structure (by ref)"))
  (if (not (`self.DoorsOpen?`))
    (`self.OpenDoors`)
    (set `self.DoorsOpen?` true)))

(event `self.Box.OnComponentEndOverlap`
  (params (OverlappedComponent :type "PrimitiveComponent Object Reference") (OtherActor :type "Actor Object Reference") (OtherComp :type "PrimitiveComponent Object Reference") (OtherBodyIndex :type Integer))
  (`KismetSystemLibrary.RetriggerableDelay` 2.0)
  (`self.CloseDoors`)
  (`KismetSystemLibrary.Delay` 1.0)
  (set `self.DoorsOpen?` false))

(event `OpenDoors`
  (`|ExecutionSequence`
    (:`then_0`
      (bind (_direction _newtrack_1) (`Timeline|OpenLeft` :!via `PlayFromStart`)
        (:`Update`
          (`SceneComponent.K2_SetRelativeLocation` (`self.SM_AutoDoorLeft`) _newtrack_1 false false))))
    (:`then_1`
      (bind (_direction_2 _newtrack_1_2) (`Timeline|OpenRight` :!via `PlayFromStart`)
        (:`Update`
          (`SceneComponent.K2_SetRelativeLocation` (`self.SM_AutoDoorRight`) _newtrack_1_2 false false))))))

(event `CloseDoors`
  (`|ExecutionSequence`
    (:`then_0`
      (bind (_direction _newtrack_1) (`Timeline|CloseLeft` :!via `ReverseFromEnd`)
        (:`Update`
          (`SceneComponent.K2_SetRelativeLocation` (`self.SM_AutoDoorLeft`) _newtrack_1 false false))))
    (:`then_1`
      (bind (_direction_2 _newtrack_1_2) (`Timeline|CloseRight` :!via `ReverseFromEnd`)
        (:`Update`
          (`SceneComponent.K2_SetRelativeLocation` (`self.SM_AutoDoorRight`) _newtrack_1_2 false false))))))

(fn `UserConstructionScript`)