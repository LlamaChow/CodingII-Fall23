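; Security camera actor that spots the third-person player character and sends guards to investigate.
; AI Perception updates start a short delay, then a delayed loop repeatedly dispatches guards and draws a debug box while the stimulus reads as sensed.
; Each dispatch sends the first non-busy guard from its list to the detected character's location, along with the camera's patrol points.
; Debug prints trace detection; Pawn Sensing events only print.
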(event `self.PawnSensing.OnSeePawn`
  (params (Pawn :type "Pawn Object Reference"))
  (`KismetSystemLibrary.PrintString` "I Can See A Pawn"))

(event `self.PawnSensing.OnComponentActivated`
  (params (Component :type "ActorComponent Object Reference") (bReset :type Boolean))
  (`KismetSystemLibrary.PrintString` "Hello"))

(event `self.AIPerception.OnTargetPerceptionUpdated`
  (params (Actor :type "Actor Object Reference") (Stimulus :type "AIStimulus Structure"))
  (bind (_age _expirationage _strength _stimuluslocation _receiverlocation _tag _bsuccessfullysensed) (break `AIStimulus` Stimulus))
  (cast `/Game/ThirdPerson/Blueprints/BP_ThirdPersonCharacter` Actor)
  (`KismetSystemLibrary.PrintString` "I Can See")
  (if _bsuccessfullysensed
    (`KismetSystemLibrary.PrintString` "The Pawn is in Front of Me")
    (`KismetSystemLibrary.Delay` 0.5) ; This could be replaced with a heat timer that builds up and can cool down
    (if _bsuccessfullysensed :!label _label
      (`KismetSystemLibrary.PrintString` "Calling Guards")
      (`self.DispatchGuard`)
      (`KismetSystemLibrary.DrawDebugBox` (`self.K2_GetActorLocation` Actor) (0.0 0.0 0.0) (struct :`R` 0.841667 :`B` 0.261922 :`A` 1.0) (struct) 10.0 25.0)
      (`KismetSystemLibrary.Delay` 0.5) ; This is here to not crash the game lmao
      (goto _label))
    (else
      (`KismetSystemLibrary.PrintString` "The Pawn Escaped"))))

(event `DispatchGuard`
  (for _array_element (`self.SecurityGuards`)
    (if (not (`/Game/GD3/Blueprints/Camera-Guard/BP_AIGuard.IsBusy` _array_element))
      (`/Game/GD3/Blueprints/Camera-Guard/BP_AIGuard.Investigate` _array_element (`self.K2_GetActorLocation` (stale `self.AIPerception.OnTargetPerceptionUpdated` Actor)) (`self.CameraPatrolPoints`))
      (break)))
  (`KismetSystemLibrary.PrintString` "No More Guards To Send"))

(fn `UserConstructionScript`)