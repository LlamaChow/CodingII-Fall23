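; BP_Singleton is a manager that saves per-level progress and tracks security guards.
; Save writes collected objects and defeated guards to an SG_Objects slot named after the current level, and DeleteSave clears that slot.
; Load empties both tracking arrays and destroys the saved actors, with guard removal nested inside the collected-object loop.
; RemoveGuardFromList moves guards from active to defeated, while ResetGuards calls TPGuardReset on active ones.
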(event `Load`
  (`KismetSystemLibrary.PrintString` "Doing The Loading Thing")
  (`KismetSystemLibrary.Delay` 0.2)
  (bind _returnvalue (`GameplayStatics.GetCurrentLevelName` true))
  (`KismetArrayLibrary.Array_Clear` (`self.PreviouslyCollectedObjs`))
  (`KismetArrayLibrary.Array_Clear` (`self.DefeatedSecurityGuards`))
  (`KismetSystemLibrary.PrintString` (`KismetStringLibrary.Concat_StrStr` "Starting Load in Level " _returnvalue " wish me luck"))
  (bind _returnvalue_2 (`GameplayStatics.DoesSaveGameExist` _returnvalue))
  (if _returnvalue_2
    (bind _returnvalue_3 (`GameplayStatics.LoadGameFromSlot` _returnvalue))
    (bind _assg_objects (cast `/Game/GD3/Blueprints/Lesson1/SG_Objects` _returnvalue_3))
    (set `self.As SG Objects` _assg_objects)
    (for _array_element (`/Game/GD3/Blueprints/Lesson1/SG_Objects.CollectedObjs` _assg_objects)
      (`Actor.K2_DestroyActor` _array_element)
      (for _array_element_2 (`/Game/GD3/Blueprints/Lesson1/SG_Objects.RemovedGuards` _assg_objects)
        (`Actor.K2_DestroyActor` _array_element_2)))))

(event `Save`
  (`KismetSystemLibrary.PrintString` "Doing The Save Thing")
  (bind _returnvalue (`GameplayStatics.GetCurrentLevelName` true))
  (bind _returnvalue_2 (`GameplayStatics.DoesSaveGameExist` _returnvalue))
  (if _returnvalue_2
    (bind _returnvalue_3 (`GameplayStatics.LoadGameFromSlot` _returnvalue))
    (set `self.SaveSubclass` _returnvalue_3)
    (else
      (bind _returnvalue_4 (`GameplayStatics.CreateSaveGameObject` "/Game/GD3/Blueprints/Lesson1/SG_Objects.SG_Objects_C"))
      (set `self.SaveSubclass` _returnvalue_4)))
  (bind _assg_objects (cast `/Game/GD3/Blueprints/Lesson1/SG_Objects` (`self.SaveSubclass`)))
  (set `/Game/GD3/Blueprints/Lesson1/SG_Objects.CollectedObjs` (`self.PreviouslyCollectedObjs`) _assg_objects)
  (set `/Game/GD3/Blueprints/Lesson1/SG_Objects.RemovedGuards` (`self.DefeatedSecurityGuards`) _assg_objects)
  (bind _returnvalue_5 (`GameplayStatics.GetCurrentLevelName` true))
  (`GameplayStatics.SaveGameToSlot` _assg_objects _returnvalue_5)
  (`KismetSystemLibrary.PrintString` "Did The Save Thing"))

(event `DeleteSave`
  (bind _returnvalue (`GameplayStatics.GetCurrentLevelName` true))
  (bind _returnvalue_2 (`GameplayStatics.DoesSaveGameExist` _returnvalue))
  (if _returnvalue_2
    (`GameplayStatics.DeleteGameInSlot` _returnvalue)
    (`KismetSystemLibrary.PrintString` "Save Deleted")
    (else
      (`KismetSystemLibrary.PrintString` "No Save Game Exists"))))

(event `Reset Guards`
  (bind _returnvalue (`self.GuardCheckValid`))
  (if _returnvalue
    (for _array_element (`self.AllSecurityGuards`) :!label _label
      (`/Game/GD3/Blueprints/Camera-Guard/BP_AIGuard.TPGuardReset` _array_element)
      (goto _label))))

(event `RemoveGuardFromList`
  (params (RemovalTarget :type "/Game/GD3/Blueprints/Camera-Guard/BP_AIGuard Object Reference"))
  (`KismetArrayLibrary.Array_RemoveItem` (`self.AllSecurityGuards`) RemovalTarget)
  (`KismetArrayLibrary.Array_Add` (`self.DefeatedSecurityGuards`) RemovalTarget))

(fn `GuardCheckValid`
  (returns (ReturnValue :type Boolean))
  (if (`KismetArrayLibrary.Array_IsValidIndex` (`self.AllSecurityGuards`))
    (return true)
    (else
      (return false))))