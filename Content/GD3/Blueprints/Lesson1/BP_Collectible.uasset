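; BP_Collectible is a pickup actor that adds to the score when something overlaps its Collider.
; AddScore casts the game instance to BP_Singleton, increments its Score and adds the pickup's own reference to PreviouslyCollectedObjs.
; It then destroys the actor, and the overlap event also calls DestroyActor afterwards.
; The overlap does not check which actor triggered it.
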(event `self.Collider.OnComponentBeginOverlap`
  (params (OverlappedComponent :type "PrimitiveComponent Object Reference") (OtherActor :type "Actor Object Reference") (OtherComp :type "PrimitiveComponent Object Reference") (OtherBodyIndex :type Integer) (bFromSweep :type Boolean) (SweepResult :type "HitResult Structure (by ref)"))
  (`self.Add Score`)
  (`self.K2_DestroyActor`))

(fn `Add Score`
  (bind _asbp_singleton (cast `/Game/GD3/Blueprints/Lesson1/BP_Singleton` (`GameplayStatics.GetGameInstance`)))
  (`/Engine/EditorBlueprintResources/StandardMacros.IncrementInt` (`/Game/GD3/Blueprints/Lesson1/BP_Singleton.Score` _asbp_singleton)
    (:`  `
      (`KismetArrayLibrary.Array_Add` (`/Game/GD3/Blueprints/Lesson1/BP_Singleton.PreviouslyCollectedObjs` _asbp_singleton) self)
      (`self.K2_DestroyActor`))))

(fn `UserConstructionScript`)